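; BP_Button is a clickable world button that tells its connected Nest to spawn a fox with the button's assigned BehaviorNumber.
; A click also plays a timeline that moves the cube along Z as a pressing animation.
; Cursor hover toggles the cube's custom depth and stencil value to control an outline highlight.
; The construction script writes BehaviorNumber onto a TextRender label.
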(event OnBeginCursorOver(Cube)
  (params (TouchedComponent :type Primitive%20Component%20Object%20Reference))
  (bind _cube (Variables|Default|GetCube))
  ;[1 1 1] Outline Control
  (Rendering|SetRenderCustomDepth _cube true)
  (Rendering|SetCustomDepthStencilValue _cube 2))

(event OnEndCursorOver(Cube)
  (params (TouchedComponent :type Primitive%20Component%20Object%20Reference))
  (bind _cube (Variables|Default|GetCube))
  ;[1 1 1] Outline Control
  (Rendering|SetRenderCustomDepth _cube false)
  (Rendering|SetCustomDepthStencilValue _cube 0))

(event EventBeginPlay)

(event Collision|EventActorBeginOverlap
  (params (OtherActor :type Actor%20Object%20Reference)))

(event EventTick
  (params (DeltaSeconds :type Float%20%28single-precision%29)))

(event MouseInput|EventActorOnClicked
  (params (ButtonPressed :type Key%20Structure :default "None"))
  ;[1 1 1] Spawn Fox From The Connected Nest
  (Default|SpawnFox (Utilities|ResolveSoftReference (Variables|Default|GetNest)) (Variables|Default|GetBehaviorNumber))
  ;[1 1 1] Button Pressing Animation
  (bind _z_minus (Timeline|Pressing%20Animation PlayFromStart)
    (:Update
      (Transformation|SetRelativeLocation (Variables|Default|GetCube) (Math|Vector|MakeVector 0.0 0.0 _z_minus) false false))))

(fn ConstructionScript
  (Rendering|Components|TextRender|SetText (Variables|Default|GetTextRender) (Utilities|Text|ToText(Integer) (Variables|Default|GetBehaviorNumber))))