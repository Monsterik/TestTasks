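; BP_Fox is an AI-moved fox character that travels to a goal using one of three movement behaviours, each exposed as a custom event.
; It moves directly, stops and starts by toggling max walk speed, or periodically backtracks by alternating move orders between goal and home.
; Delay-driven loops run until GoalAchived is set on arrival, which plays win sound and particles; spawning has its own effects.
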(event Custom|Move%20To%20Destination%20Reversing
  (params (Goal%20Destination :type Vector) (Home%20Destination :type Vector))
  ;[1 1 1] Third Behaviour
  (AI|AIMoveTo self Goal%20Destination 0 1e+01 false :!label _label
    (:then
      (Utilities|FlowControl|Delay 1.0)
      (if (not (Variables|Default|GetGoal%20Achived))
        (AI|AIMoveTo self Home%20Destination 0 1e+01 false
          (:then
            (Utilities|FlowControl|Delay 0.5)
            (goto _label)))))
    (:OnSuccess
      (Variables|Default|SetGoal%20Achived true)
      (Audio|PlaySound2D "/Game/TestTaskUE/Art/Sounds/A_Win.A_Win" 2.0 1.0 0.0 0 0)
      (Effects|SpawnEmitteratLocation "/Game/TestTaskUE/Art/Particles/Flares/P_Success.P_Success" (Transformation|GetActorLocation) "0, 0, 0" "0.500000,0.500000,0.500000"))))

(event Custom|Move%20To%20Destination%20Simple
  (params (Goal%20Destination :type Vector))
  ;[1 1 1] First Behaviour
  (AI|AIMoveTo self Goal%20Destination 0 1e+01 false
    (:OnSuccess
      (Variables|Default|SetGoal%20Achived true)
      (Audio|PlaySound2D "/Game/TestTaskUE/Art/Sounds/A_Win.A_Win" 2.0 1.0 0.0 0 0)
      (Effects|SpawnEmitteratLocation "/Game/TestTaskUE/Art/Particles/Flares/P_Success.P_Success" (Transformation|GetActorLocation) "0, 0, 0" "0.500000,0.500000,0.500000"))))

(event Custom|Move%20To%20Destination%20Stopping
  (params (Goal%20Destination :type Vector))
  ;[1 1 1] Second Behaviour
  (AI|AIMoveTo self Goal%20Destination 0 1e+01 false
    (:then
      (if (not (Variables|Default|GetGoal%20Achived)) :!label _label
        (Variables|/Script/Engine.CharacterMovementComponent|SetMaxWalkSpeed (Variables|Character|GetCharacterMovement) 1.5e+02)
        (Utilities|FlowControl|Delay 1.0)
        (Variables|/Script/Engine.CharacterMovementComponent|SetMaxWalkSpeed (Variables|Character|GetCharacterMovement) 0.0)
        (Utilities|FlowControl|Delay 0.5)
        (goto _label)))
    (:OnSuccess
      (Variables|Default|SetGoal%20Achived true)
      (Audio|PlaySound2D "/Game/TestTaskUE/Art/Sounds/A_Win.A_Win" 2.0 1.0 0.0 0 0)
      (Effects|SpawnEmitteratLocation "/Game/TestTaskUE/Art/Particles/Flares/P_Success.P_Success" (Transformation|GetActorLocation) "0, 0, 0" "0.500000,0.500000,0.500000"))))

(event EventBeginPlay
  ;[1 1 1] Spawning Sound And Particles
  (Audio|PlaySound2D "/Game/TestTaskUE/Art/Sounds/A_Start.A_Start" 1.0 0.8 0.0 0 0)
  (Effects|SpawnEmitteratLocation "/Game/TestTaskUE/Art/Particles/Flares/P_Spawn.P_Spawn" (Transformation|GetActorLocation) "0, 0, 0" "0.500000,0.500000,0.500000"))

(fn ConstructionScript)