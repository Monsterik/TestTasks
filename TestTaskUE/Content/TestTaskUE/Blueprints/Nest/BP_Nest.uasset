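; BP_Nest is a nest that spawns BP_Fox AI pawns and sends them toward its linked NestDestination.
; The SpawnFox event spawns a fox at SpawnPoint and takes a one-based BehaviorID to select simple, stopping or reversing movement.
; Each mode calls the matching movement function on the fox with the destination's location, and reversing also passes the spawn point as home.
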(event Custom|Spawn%20Fox
  (params (BehaviorID :type Integer))
  (bind _nest_destination (Variables|Default|GetNest%20Destination))
  (bind _output (Utilities|ResolveSoftReference _nest_destination))
  (bind _returnvalue (Transformation|GetActorLocation _output))
  ;[1 1 1] Spawn Fox
  (bind _returnvalue_2 (AI|SpawnAIFromClass "/Game/TestTaskUE/Blueprints/Fox/BP_Fox.BP_Fox_C" 0 (Transformation|GetWorldLocation (Variables|Default|GetSpawnPoint)) "0, 0, 0" false 0))
  (bind _asbp_fox (Utilities|Casting|CastToBP_Fox _returnvalue_2))
  ;[1 1 1] Activate Fox Behaviour Based On Recieved ID And Send Connected To The Nest Destination
  (switch int (- BehaviorID 1)
    (:0
      (Default|MovetoDestinationSimple _asbp_fox _returnvalue))
    (:1
      (Default|MovetoDestinationStopping _asbp_fox _returnvalue))
    (:2
      (Default|MovetoDestinationReversing _asbp_fox _returnvalue (Transformation|GetWorldLocation (Variables|Default|GetSpawnPoint))))))

(fn ConstructionScript)